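; MainCharacter is the player character for a twin-stick shooter, armed with a wand and aimed with the mouse.
; On BeginPlay it spawns a Weapon attached to the Wandtemp component and adds the TwinStickHUD to the viewport.
; Input moves it along world axes and pulls or releases the weapon trigger, while Tick yaws it toward the cursor hit point.
; AffectHealth recalculates health and destroys weapon and character on death.
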(event `self.ReceiveBeginPlay`
  (bind _wandtemp (`self.Wandtemp`))
  (`|ExecutionSequence`
    (:`then_0`
      (bind _returnvalue (`|SpawnActorFromClass` "/Game/Blueprints/Weapon.Weapon_C" (`SceneComponent.K2_GetComponentToWorld` _wandtemp) "Undefined" "OverrideRootScale" null null))
      (bind _output_get (set `self.Weapon` _returnvalue))
      (`self.K2_AttachToComponent` _output_get _wandtemp "None" "SnapToTarget" "KeepRelative" "KeepWorld" true))
    (:`then_1`
      (bind _returnvalue_2 (`|CreateWidget` "/Game/Blueprints/TwinStickHUD.TwinStickHUD_C"))
      (`UserWidget.AddToViewport` _returnvalue_2 0))))

(event `InputAxis|MoveRight`
  (params (AxisValue :type "Float (single-precision)"))
  ;[1 1 1] Movement
  (`self.AddMovementInput` (0.0 1.0 0.0) AxisValue))

(event `InputAction|ShootWand`
  (params (Key :type "Key Structure"))
  (bind _weapon (`self.Weapon`))
  ;[1 1 1] Weapon, firing key
  (:`Pressed`
    (`/Game/Blueprints/Weapon.PullTrigger` _weapon))
  (:`Released`
    (`/Game/Blueprints/Weapon.ReleaseTrigger` _weapon)))

(event `InputAxis|MoveUp`
  (params (AxisValue :type "Float (single-precision)"))
  ;[1 1 1] Movement
  (`self.AddMovementInput` (1.0 0.0 0.0) AxisValue))

(event `self.ReceiveTick`
  (params (DeltaSeconds :type "Float (single-precision)"))
  ;[1 1 1] Rotation with mouse
  (`self.K2_SetActorRelativeRotation` (`KismetMathLibrary.MakeRotator` 0.0 0.0 (.yaw (`KismetMathLibrary.FindLookAtRotation` (`self.K2_GetActorLocation`) (`.Location` (`GameplayStatics.BreakHitResult` (`PlayerController.GetHitResultUnderCursorByChannel` (`GameplayStatics.GetPlayerController` 0) "TraceTypeQuery1" true))))))))

(event `/Game/Blueprints/iDamageable.AffectHealth`
  (params (Delta :type "Float (single-precision)"))
  (`self.CalculateHealth` Delta)
  (if (`self.IsDead`)
    (`self.K2_DestroyActor` (`self.Weapon`))
    (`self.K2_DestroyActor` self)))

(fn `UserConstructionScript`
  (`parent.UserConstructionScript`))