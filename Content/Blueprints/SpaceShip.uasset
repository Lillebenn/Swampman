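; SpaceShip is a player-controlled ship pawn with sideways movement, look-driven rotation and a spawned weapon.
; BeginPlay spawns the weapon at the Guntemp component and attaches it there, and the ShootGun press and release pull and release its trigger.
; MoveRight adds movement along world Y.
; LookForward and LookRight share one path that sets controller rotation from an axis-built vector when its length is non-zero.
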(event `self.ReceiveBeginPlay`
  (bind _guntemp (`self.Guntemp`))
  ;[1 1 1] Part of the weapon shooting
  (`|ExecutionSequence`
    (:`then_0`
      (bind _returnvalue (`|SpawnActorFromClass` "/Game/Blueprints/Weapon.Weapon_C" (`SceneComponent.K2_GetComponentToWorld` _guntemp) "Undefined" "OverrideRootScale" null null))
      (bind _output_get (set `self.Weapon` _returnvalue))
      (`self.K2_AttachToComponent` (`self.Weapon`) _guntemp "None" "SnapToTarget" "KeepRelative" "KeepWorld" true)
      (`self.K2_AttachToComponent` _output_get _guntemp "None" "SnapToTarget" "KeepRelative" "KeepWorld" true))))

(event `InputAxis|MoveRight`
  (params (AxisValue :type "Float (single-precision)"))
  ;[1 1 1] Movement
  (`self.AddMovementInput` (0.0 1.0 0.0) AxisValue))

(event `InputAxis|LookForward`
  (params (AxisValue :type "Float (single-precision)"))
  ;[1 1 1] Rotation
  (bind _returnvalue (`KismetMathLibrary.MakeVector` AxisValue (stale `InputAxis|LookRight` AxisValue)))
  (if (> (`KismetMathLibrary.VSize` _returnvalue) 0.0) :!label _label
    (`Controller.SetControlRotation` (`self.GetController`) (`KismetMathLibrary.Conv_VectorToRotator` _returnvalue))))

(event `InputAction|ShootGun`
  (params (Key :type "Key Structure"))
  (bind _weapon (`self.Weapon`))
  ;[1 1 1] When does the weapon fire
  (:`Pressed`
    (`/Game/Blueprints/Weapon.PullTrigger` _weapon))
  (:`Released`
    (`/Game/Blueprints/Weapon.ReleaseTrigger` _weapon)))

(event `InputAxis|LookRight`
  (params (AxisValue :type "Float (single-precision)"))
  ;[1 1 1] Rotation
  (goto _label))

(fn `UserConstructionScript`
  (`parent.UserConstructionScript`))