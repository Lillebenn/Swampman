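; Invader enemy Blueprint that repeatedly damages the MainCharacter while overlapping it, and can itself be hurt and killed.
; Overlap stores the hero and starts a looping DamageTheHero timer at AttacksPerSecond, calling AffectHealth on the hero.
; Any actor ending overlap clears the timer, as the hero comparison is left unconnected.
; Its own AffectHealth event runs CalculateHealth and destroys the actor once IsDead is set.
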(event `/Game/Blueprints/iDamageable.AffectHealth`
  (params (Delta :type "Float (single-precision)"))
  (`self.CalculateHealth` Delta)
  (if (`self.IsDead`)
    (`self.K2_DestroyActor`)))

(event `self.ReceiveActorBeginOverlap`
  (params (OtherActor :type "Actor Object Reference"))
  (bind _asmain_character (cast `/Game/Blueprints/MainCharacter` OtherActor))
  (set `self.Hero` _asmain_character)
  (`KismetSystemLibrary.K2_SetTimer` null "DamageTheHero" (/ 1.0 (`self.Attacks Per Second`)) true))

(event `self.ReceiveActorEndOverlap`
  (params (OtherActor :type "Actor Object Reference"))
  (if true
    (`KismetSystemLibrary.K2_ClearTimer` null "DamageTheHero")))

(event `DamageTheHero`
  (`/Game/Blueprints/MainCharacter.AffectHealth` (`self.Hero`) (`self.Damage`)))

(fn `UserConstructionScript`
  (`parent.UserConstructionScript`))